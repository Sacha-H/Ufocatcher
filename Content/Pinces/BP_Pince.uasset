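; BP_Pince is the player-controlled claw machine pawn, viewed through a level camera.
; When idle, the grab input decrements money and starts a round, updating the WB_UI widget; during play, Enhanced Input moves the claw until a grab begins.
; Timelines lower or raise it with randomized spin, then return it to start, ending the round.
; MoveBras toggles the arms by flipping physics thrusters 180 degrees; Tick draws a downward debug trace.
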(event Input|EnhancedActionEvents|EnhancedInputActionIA_Move
  (params (ActionValue :type Vector%202D%20Structure) (ElapsedSeconds :type Float%20%28double-precision%29) (TriggeredSeconds :type Float%20%28double-precision%29) (InputAction :type Input%20Action%20Object%20Reference :default "/Game/Pinces/Input/Input/IA_Move.IA_Move"))
  (if (and (not (Variables|Default|GetIs%20grabing)) (Variables|Default|GetIsPlaying))
    (Pawn|Input|AddMovementInput (Transformation|GetActorRightVector) (.x ActionValue) false)
    (Pawn|Input|AddMovementInput (Transformation|GetActorForwardVector) (.y ActionValue) false)))

(event Input|EnhancedActionEvents|EnhancedInputActionIA_Grab
  (params (ActionValue :type Boolean) (ElapsedSeconds :type Float%20%28double-precision%29) (TriggeredSeconds :type Float%20%28double-precision%29) (InputAction :type Input%20Action%20Object%20Reference :default "/Game/Pinces/Input/Input/IA_Grab.IA_Grab"))
  (bind _returnvalue (Transformation|GetActorRotation))
  (bind _returnvalue_2 (Transformation|GetActorLocation))
  (bind _ui (Variables|Default|GetUI))
  (:Started
    (if (Variables|Default|GetIsPlaying)
      (if (not (Variables|Default|GetIs%20grabing))
        (Variables|Default|SetIs%20grabing true)
        (Variables|Default|SetRandomRotation (Math|Random|RandomFloatinRange 0.8 2.0))
        (bind (_direction _newtrack_0 _rotate) (Timeline|TimelineGrabing PlayFromStart)
          (:Update
            (Transformation|SetActorLocation (Math|Vector|MakeVector (.x _returnvalue_2) (.y _returnvalue_2) (Math|Float|Lerp (Variables|Default|GetInitialValueZ) 5e+02 _newtrack_0)) false false)
            (Transformation|SetActorRotation (Math|Rotator|MakeRotator (.roll _returnvalue) (.pitch _returnvalue) (+ (* _rotate (Variables|Default|GetRandomRotation)) (.yaw _returnvalue)))))
          (:Finished
            (Variables|Default|SetResetLocation (Transformation|GetActorLocation))
            (Variables|Default|SetResetRotation (Transformation|GetActorRotation))
            (bind _newtrack_0_2 (Timeline|TimelineResetPosition PlayFromStart)
              (:Update
                (Transformation|SetActorLocation (Math|Vector|Lerp(Vector) (Variables|Default|GetResetLocation) (Variables|Default|GetinitialLocation) _newtrack_0_2) false false)
                (Transformation|SetActorRotation (Math|Rotator|Lerp(Rotator) (Variables|Default|GetResetRotation) (Variables|Default|GetInitialRotation) _newtrack_0_2 true)))
              (:Finished
                (Variables|Default|SetIs%20grabing false)
                (CallFunction|MoveBras (Variables|Default|GetPhysicsThruster))
                (CallFunction|MoveBras (Variables|Default|GetPhysicsThruster1))
                (CallFunction|MoveBras (Variables|Default|GetPhysicsThruster2))
                (Variables|Default|SetIsPlaying false)
                (Default|EventSetPlayingVisibility (Variables|Default|GetUI) "Visible"))))
          (:NewTrack_1
            (CallFunction|MoveBras (Variables|Default|GetPhysicsThruster))
            (CallFunction|MoveBras (Variables|Default|GetPhysicsThruster1))
            (CallFunction|MoveBras (Variables|Default|GetPhysicsThruster2)))))
      (else
        (bind _result (Math|Integer|DecrementInt (Variables|Default|GetMoneyValue))
          (:%20%20
            (Variables|Default|SetIsPlaying true)
            (Default|EventSetMoney _ui _result)
            (Default|EventSetPlayingVisibility _ui "Hidden")))))))

(event Input|EnhancedActionEvents|EnhancedInputActionIA_Debug
  (params (ActionValue :type Boolean) (ElapsedSeconds :type Float%20%28double-precision%29) (TriggeredSeconds :type Float%20%28double-precision%29) (InputAction :type Input%20Action%20Object%20Reference :default "/Game/Pinces/Input/Input/IA_Debug.IA_Debug")))

(event EventBeginPlay
  (bind _asplayer_controller (Utilities|Casting|CastToPlayerController (Pawn|GetController)))
  (Utilities|IsValid (PlayerController|LocalPlayerSubsystems|GetEnhancedInputLocalPlayerSubsystem _asplayer_controller)
    (:Is%20Valid
      (Input|AddMappingContext (PlayerController|LocalPlayerSubsystems|GetEnhancedInputLocalPlayerSubsystem _asplayer_controller) "/Game/Pinces/Input/NewInputMappingContext.NewInputMappingContext" 0 "(bIgnoreAllPressedKeysUntilRelease=True,bForceImmediately=False,bNotifyUserSettings=False)")
      (bind _returnvalue (Actor|GetActorOfClass "/Script/Engine.CameraActor"))
      (Game|Player|SetViewTargetwithBlend _asplayer_controller _returnvalue 0.0 "VTBlend_Linear" 0.0 false)
      (Variables|Default|SetInitialValueZ (.z (Transformation|GetActorLocation)))
      (Components|Timeline|SetPlayRate (Variables|Default|GetTimelineGrabing) 0.2)
      (Components|Timeline|SetPlayRate (Variables|Default|GetTimelineResetPosition) 0.4)
      (Variables|Default|SetinitialLocation (Transformation|GetActorLocation))
      (Variables|Default|SetInitialRotation (Transformation|GetActorRotation))
      (bind _returnvalue_2 (UserInterface|CreateWidget "/Game/Winget/WB_UI.WB_UI_C"))
      (bind _output_get (Variables|Default|SetUI _returnvalue_2))
      (UserInterface|Viewport|AddtoViewport _output_get 0)
      (Default|EventSetMoney (Variables|Default|GetUI) (Variables|Default|GetMoneyValue)))))

(event Collision|EventActorBeginOverlap
  (params (OtherActor :type Actor%20Object%20Reference)))

(event EventTick
  (params (DeltaSeconds :type Float%20%28single-precision%29))
  (bind _returnvalue (Transformation|GetActorLocation))
  (Collision|LineTraceByChannel _returnvalue (+ _returnvalue (* (Transformation|GetActorUpVector) -1e+03)) "TraceTypeQuery1" false 0 "ForOneFrame"))

(fn ConstructionScript)

(fn MoveBras
  (params (Target :type Scene%20Component%20Object%20Reference))
  (bind _relativerotation (Variables|/Script/Engine.SceneComponent|GetRelativeRotation Target))
  (bind (_roll _pitch _yaw) (Math|Rotator|BreakRotator _relativerotation))
  (Transformation|SetRelativeRotation (Variables|Default|GetPhysicsThruster) (Math|Rotator|MakeRotator _roll (+ _pitch 1.8e+02) _yaw) false false))